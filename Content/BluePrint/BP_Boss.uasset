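; BP_Boss is an enemy boss that moves along a timeline-driven offset from its starting location.
; Projectile hits lower its HP, switching body and eye materials to attack versions at a threshold; at zero it restores base body materials, then explodes after a short delay.
; Hitting the first-person character makes it explode immediately and damage that player, only printing HP and death.
; An older MoveComponentTo up-and-down loop remains unconnected.
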(event EventBeginPlay
  (Variables|Default|SetinitialL (Transformation|GetActorLocation))
  (bind _새_트랙_1 (Timeline|타임라인_0 Play)
    (:Update
      (Transformation|SetActorLocation (+ (Variables|Default|GetinitialL) _새_트랙_1) false false))))

(event Collision|EventHit
  (params (MyComp :type Primitive%20Component%20Object%20Reference) (Other :type Actor%20Object%20Reference) (OtherComp :type Primitive%20Component%20Object%20Reference) (bSelfMoved :type Boolean) (HitLocation :type Vector :default "0, 0, 0") (HitNormal :type Vector :default "0, 0, 0") (NormalImpulse :type Vector :default "0, 0, 0") (Hit :type Hit%20Result%20Structure%20%28by%20ref%29))
  (bind _staticmesh (Variables|Default|GetStaticMesh))
  (bind _staticmesh_2 (Variables|Default|GetStaticMesh))
  (Utilities|Casting|CastToFirstPersonProjectileAttack Other
    (:then
      (Variables|Default|SetEnemyHP (- (Variables|Default|GetEnemyHP) 1e+01))
      (if (<= (Variables|Default|GetEnemyHP) 5e+01)
        (Rendering|Material|SetMaterial _staticmesh 0 "/Game/Enemy/M_EnemyBodyAttack.M_EnemyBodyAttack")
        (Rendering|Material|SetMaterial _staticmesh 11 "/Game/Enemy/M_EnemyBodyAttack.M_EnemyBodyAttack")
        (Rendering|Material|SetMaterial _staticmesh 5 "/Game/Enemy/M_EnemyEyeAttack.M_EnemyEyeAttack")
        (if (<= (Variables|Default|GetEnemyHP) 0.0)
          (Rendering|Material|SetMaterial _staticmesh_2 0 "/Game/FirstPerson/Meshes/BaseMaterial.BaseMaterial")
          (Rendering|Material|SetMaterial _staticmesh_2 11 "/Game/FirstPerson/Meshes/BaseMaterial.BaseMaterial")
          (Rendering|Material|SetMaterial _staticmesh_2 5 "/Game/Enemy/M_EnemyEyeAttack.M_EnemyEyeAttack")
          (Utilities|FlowControl|Delay 0.5)
          (Effects|SpawnEmitteratLocation "/Game/StarterContent/Particles/P_Explosion.P_Explosion" (Transformation|GetActorLocation) "0, 0,0.000000")
          (Actor|DestroyActor))))
    (:CastFailed
      (bind _asfirst_person_character (Utilities|Casting|CastToFirstPersonCharacter Other))
      (Effects|SpawnEmitteratLocation "/Game/StarterContent/Particles/P_Explosion.P_Explosion" (Transformation|GetActorLocation _asfirst_person_character))
      (Actor|DestroyActor)
      (Variables|/Game/FirstPersonBP/Blueprints/FirstPersonCharacter.FirstPersonCharacter_C|SetMYHP _asfirst_person_character (- (Variables|/Game/FirstPersonBP/Blueprints/FirstPersonCharacter.FirstPersonCharacter_C|GetMYHP _asfirst_person_character) 25.0))
      (Development|PrintString (Utilities|String|ToString(Float) (Variables|/Game/FirstPersonBP/Blueprints/FirstPersonCharacter.FirstPersonCharacter_C|GetMYHP _asfirst_person_character)))
      (if (<= (Variables|/Game/FirstPersonBP/Blueprints/FirstPersonCharacter.FirstPersonCharacter_C|GetMYHP _asfirst_person_character) 0.0)
        (Development|PrintString "Dead")))))

(fn ConstructionScript)